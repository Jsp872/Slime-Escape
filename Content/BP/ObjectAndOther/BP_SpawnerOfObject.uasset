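; BP_SpawnerOfObject spawns an object and can later return it to a spawn point.
; On BeginPlay it spawns ActorToSpawn at its root transform and, if that is a BP_PortalJumpObject, stores it and sets itself as its Spawner.
; RespawnObject reuses that stored actor, moving its root to the SpawnOfObject component's location and rotation at a fixed half scale instead of spawning a new one.
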(event EventBeginPlay
  (bind _returnvalue (Game|SpawnActorfromClass (Variables|Default|GetActorToSpawn) (Transformation|GetWorldTransform (Variables|Default|GetDefaultSceneRoot)) "Undefined" "MultiplyWithRoot" 0 0))
  (bind _asbp_portal_jump_object (Utilities|Casting|CastToBP_PortalJumpObject _returnvalue))
  (Variables|Default|SetObjectSpawn _asbp_portal_jump_object)
  (Variables|/Game/BP/ObjectAndOther/BP_PortalJumpObject.BP_PortalJumpObject_C|SetSpawner _asbp_portal_jump_object self))

(event EventRespawnObject
  (bind _spawnofobject (Variables|Default|GetSpawnOfObject))
  (bind _returnvalue (Transformation|GetWorldTransform _spawnofobject))
  (Transformation|SetWorldTransform (Variables|/Script/Engine.Actor|GetRootComponent (Variables|Default|GetObjectSpawn)) (Math|Transform|MakeTransform (.location _returnvalue) (.rotation _returnvalue) "0.500000,0.500000,0.500000") false false))

(fn ConstructionScript)