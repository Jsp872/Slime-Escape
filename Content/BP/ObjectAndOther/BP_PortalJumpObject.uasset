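; A physics-agnostic portal object that shows a duplicate mesh at the exit door while it passes through a portal.
; Activation unhides SMCopy and attaches it to the exit door.
; Each Tick mirrors SMObject's entry-relative transform onto the copy, rotating only the location 180 degrees around the entry door's up vector.
; Deactivation hides the copy and moves SMObject to its transform; the not-in-portal variant then zeroes SMObject's relative location.
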(event EventBeginPlay)

(event Collision|EventActorBeginOverlap
  (params (OtherActor :type Actor%20Object%20Reference)))

(event EventTick
  (params (DeltaSeconds :type Float%20%28single-precision%29))
  (bind _sm_object (Variables|Default|GetSM_Object))
  (bind _entry_door (Variables|Default|GetEntry%20Door))
  (bind _returnvalue (Transformation|GetWorldTransform _sm_object))
  (bind _returnvalue_2 (Transformation|GetWorldTransform _entry_door))
  (bind _returnvalue_3 (Math|Transform|MakeRelativeTransform _returnvalue _returnvalue_2))
  (if (Variables|Default|GetDuplicatedActivated)
    (Transformation|SetRelativeTransform (Variables|Default|GetSM_Copy) (Math|Transform|MakeTransform (Math|Vector|RotateVectorAroundAxis (.location _returnvalue_3) 1.8e+02 (Math|Vector|GetUpVector _entry_door)) (.rotation _returnvalue_3) (.scale _returnvalue_3)) false false)))

(event EventActivateDuplicate
  (params (EntryDoor :type Scene%20Component%20Object%20Reference) (ExitDoor :type Scene%20Component%20Object%20Reference))
  (Variables|Default|SetEntry%20Door EntryDoor)
  (Variables|Default|SetExit%20Door ExitDoor)
  (Transformation|DetachFromComponent (Variables|Default|GetSM_Copy) "KeepWorld" "KeepWorld" "KeepWorld" true)
  (Variables|Default|SetDuplicatedActivated true)
  (Development|SetHiddeninGame (Variables|Default|GetSM_Copy) false false)
  (Transformation|AttachComponentToComponent (Variables|Default|GetSM_Copy) (Variables|Default|GetExit%20Door) "None" "KeepWorld" "KeepWorld" "KeepWorld" true))

(event EventDesactivateDuplicate
  (bind _sm_copy (Variables|Default|GetSM_Copy))
  (if (Variables|Default|GetDuplicatedActivated)
    (Variables|Default|SetDuplicatedActivated false)
    (Development|SetHiddeninGame _sm_copy true false)
    (Transformation|SetWorldTransform (Variables|Default|GetSM_Object) (Transformation|GetWorldTransform _sm_copy) false true)))

(event EventDesactivateDuplicateifObjectNotinPortal
  (bind _sm_object (Variables|Default|GetSM_Object))
  (bind _sm_copy (Variables|Default|GetSM_Copy))
  (if (Variables|Default|GetDuplicatedActivated)
    (Variables|Default|SetDuplicatedActivated false)
    (Development|SetHiddeninGame _sm_copy true false)
    (Transformation|SetWorldTransform _sm_object (Transformation|GetWorldTransform _sm_copy) false false)
    (Transformation|SetRelativeLocation _sm_object "0, 0, 0" false false)))

(fn ConstructionScript)