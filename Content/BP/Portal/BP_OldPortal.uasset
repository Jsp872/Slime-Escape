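; Portal pair actor that teleports overlapping actors between two colliders via JumpPortalMessage, tracking the exit collider to prevent an immediate bounce back.
; Each tick, proxy components follow the player camera and drive the opposite scene capture's position, look-at rotation and distance-based FOV for the portal views.
; PlacePortal positions and reveals either portal, while CanPlacePortal traces four edges for a valid surface type, nudging a dummy portal to fit.
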(event OnComponentBeginOverlap(Col2)
  (params (OverlappedComponent :type Primitive%20Component%20Object%20Reference) (OtherActor :type Actor%20Object%20Reference) (OtherComp :type Primitive%20Component%20Object%20Reference) (OtherBodyIndex :type Integer) (bFromSweep :type Boolean) (SweepResult :type Hit%20Result%20Structure%20%28by%20ref%29))
  (Utilities|JumpPortalM OtherActor (Variables|Default|GetCol1) (Variables|Default|GetP1Capture) OverlappedComponent))

(event OnComponentBeginOverlap(Col1)
  (params (OverlappedComponent :type Primitive%20Component%20Object%20Reference) (OtherActor :type Actor%20Object%20Reference) (OtherComp :type Primitive%20Component%20Object%20Reference) (OtherBodyIndex :type Integer) (bFromSweep :type Boolean) (SweepResult :type Hit%20Result%20Structure%20%28by%20ref%29))
  (Utilities|JumpPortalM OtherActor (Variables|Default|GetCol2) (Variables|Default|GetP2Capture) OverlappedComponent))

(event OnComponentEndOverlap(Col1)
  (params (OverlappedComponent :type Primitive%20Component%20Object%20Reference) (OtherActor :type Actor%20Object%20Reference) (OtherComp :type Primitive%20Component%20Object%20Reference) (OtherBodyIndex :type Integer))
  (Utilities|ClearExitCollider OverlappedComponent))

(event OnComponentEndOverlap(Col2)
  (params (OverlappedComponent :type Primitive%20Component%20Object%20Reference) (OtherActor :type Actor%20Object%20Reference) (OtherComp :type Primitive%20Component%20Object%20Reference) (OtherBodyIndex :type Integer))
  (Utilities|ClearExitCollider OverlappedComponent))

(event Custom|PlacePortal
  (params (Portal :type Boolean) (NewLocation :type Vector) (NewRotation :type Rotator))
  (bind _test (Variables|Default|GetTest))
  (bind _defaultsceneroot (Variables|/Game/PortalSystem/BP_Portal.BP_Portal_C|GetDefaultSceneRoot _test))
  (if Portal
    (if (not (Rendering|IsVisible _defaultsceneroot))
      (Transformation|SetWorldLocationAndRotation _defaultsceneroot NewLocation NewRotation false false)
      (Rendering|SetVisibility (Variables|/Game/PortalSystem/BP_Portal.BP_Portal_C|GetDefaultSceneRoot (Variables|Default|GetTest)) true true))
    (else
      (Transformation|SetWorldLocationAndRotation (Variables|/Game/PortalSystem/BP_Portal.BP_Portal_C|GetDefaultSceneRoot (Variables|Default|GetTest_0)) NewLocation NewRotation false false)
      (Rendering|SetVisibility (Variables|/Game/PortalSystem/BP_Portal.BP_Portal_C|GetDefaultSceneRoot (Variables|Default|GetTest_0)) true true))))

(event EventBeginPlay)

(event Collision|EventActorBeginOverlap
  (params (OtherActor :type Actor%20Object%20Reference)))

(event EventTick
  (params (DeltaSeconds :type Float%20%28single-precision%29))
  (CallFunction|UpdateCameras))

(fn ConstructionScript)

(fn UpdateCameras
  (Transformation|SetWorldLocation (Variables|Default|GetPSimD1) (Camera|GetCameraLocation (Game|GetPlayerCameraManager 0)) false false)
  (Utilities|UpdateCaptureM (Variables|Default|GetP1Capture) (Variables|Default|GetPSimD2))
  (Utilities|UpdateCaptureM (Variables|Default|GetP2Capture) (Variables|Default|GetPSimD1))
  (return))

(fn CheckSurface
  (params (InputPin :type Scene%20Component%20Object%20Reference))
  (bind _returnvalue (Transformation|GetWorldLocation InputPin))
  (bind (_outhit _returnvalue_2) (Collision|LineTraceByChannel _returnvalue (+ _returnvalue (* (Math|Vector|GetForwardVector InputPin) 5e+01)) "TraceTypeQuery1" false 0 "ForDuration"))
  (if _returnvalue_2
    (return (Utilities|Enum|Equal(Enum) (Variables|/Script/PhysicsCore.PhysicalMaterial|GetSurfaceType (.PhysMat (Collision|BreakHitResult _outhit))) "SurfaceType1"))
    (else
      (return false))))